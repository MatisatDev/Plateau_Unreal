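; BP_Cell_Score is a bonus cell, apparently for a board game, that awards 10 points to the player it acts on.
; Its Action override calls the parent, then rewrites that player's SPlayerData entry in the game instance's PlayerList, keeping ID and cell number.
; The debug print re-reads the updated score and adds 10 again, so it shows 10 more than the stored value.
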(event EventBeginPlay
  (|CallParentFunction) ; This node is disabled and will not be called.\nDrag off pins to build functionality.
)

(event Collision|EventActorBeginOverlap
  (params (OtherActor :type Actor%20Object%20Reference))
  (|CallParentFunction OtherActor) ; This node is disabled and will not be called.\nDrag off pins to build functionality.
)

(event EventTick
  (params (DeltaSeconds :type Float%20%28single-precision%29))
  (|CallParentFunction DeltaSeconds) ; This node is disabled and will not be called.\nDrag off pins to build functionality.
)

(fn ConstructionScript
  (|CallParentFunction))

(fn Action
  (params (PlayerID :type Integer))
  (bind _as_bp_game_instance (Variables|Default|GetAs%20BP%20Game%20Instance))
  (bind _playerlist (Variables|/Game/Blueprints/BP_GameInstance.BP_GameInstance_C|GetPlayerList _as_bp_game_instance))
  (bind _output (Utilities|Array|Get(acopy) _playerlist PlayerID))
  (bind (_playerid _score _cellnumber) (Utilities|Struct|BreakS_PlayerData _output))
  (bind _returnvalue (+ _score 10))
  (|CallParentFunction PlayerID)
  (Utilities|Array|SetArrayElem _playerlist PlayerID (Utilities|Struct|MakeS_PlayerData _playerid _returnvalue _cellnumber))
  (Development|PrintString "Bonus Point")
  (Development|PrintString (Utilities|String|ToString(Integer) _returnvalue)))