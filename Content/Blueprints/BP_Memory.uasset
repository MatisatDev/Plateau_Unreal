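; BP_Memory is a clickable card for a memory minigame that flips over when selected and reports to BP_MiniGameMode.
; Clicking its Door component plays the TurnCard timeline to rotate it in yaw, with a DoOnce on the update calling TwoCardChoosen.
; When the flip finishes, the card adds itself to the game mode's CardListChoosen and calls CardVerification.
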(event OnClicked(Card)
  (params (TouchedComponent :type Primitive%20Component%20Object%20Reference) (ButtonPressed :type Key%20Structure :default "None")))

(event OnClicked(Door)
  (params (TouchedComponent :type Primitive%20Component%20Object%20Reference) (ButtonPressed :type Key%20Structure :default "None"))
  (Development|PrintString "Card Selected")
  (bind _open (Timeline|Turn%20Card Play)
    (:Update
      (Transformation|SetRelativeRotation (Variables|Default|GetDoor) (Math|Rotator|MakeRotator 0.0 0.0 _open) false false)
      (Utilities|FlowControl|DoOnce false
        (:Completed
          (Default|TwoCardChoosen? (Variables|Default|GetMiniGM_Ref)))))
    (:Finished
      (Development|PrintString "Hello")
      (Utilities|Array|Add (Variables|/Game/Blueprints/BP_MiniGameMode.BP_MiniGameMode_C|GetCard%20List%20Choosen (Variables|Default|GetMiniGM_Ref)) self)
      (Default|CardVerification (Variables|Default|GetMiniGM_Ref)))))

(event EventBeginPlay
  (bind _asbp_mini_game_mode (Utilities|Casting|CastToBP_MiniGameMode (Game|GetGameMode)))
  (Variables|Default|SetMiniGM_Ref _asbp_mini_game_mode))

(fn ConstructionScript)