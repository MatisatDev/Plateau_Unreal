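; Game mode for a memory card-matching minigame played with mouse clicks.
; On BeginPlay it spawns a BP_Memory card per CardListToSpawn entry in rows of four, assigning each its CardIndex.
; It counts picks and hides the cursor at two.
; Verification compares indices: mismatches rotate back via a reversed timeline, then restore the cursor and clear the selection, while matches have no handling here.
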(event Custom|Spawn%20Card
  (for _array_element (Variables|Default|GetCard%20List%20To%20Spawn)
    (bind _returnvalue (Game|SpawnActorfromClass "/Game/Blueprints/BP_Memory.BP_Memory_C" (Variables|Default|GetCard%20Spawn) "Undefined" "MultiplyWithRoot" 0 0))
    (Variables|/Game/Blueprints/BP_Memory.BP_Memory_C|SetCard%20Index _returnvalue _array_element)
    (Variables|Default|SetCard%20Spawn (Math|Transform|MakeTransform (Math|Vector|MakeVector (.x (.location (Variables|Default|GetCard%20Spawn))) (+ (.y (.location (Variables|Default|GetCard%20Spawn))) 2e+02) (.z (.location (Variables|Default|GetCard%20Spawn)))) "0, 0, 0" "1.000000,1.000000,1.000000"))
    (Math|Integer|IncrementInt (Variables|Default|GetSpawn%20Index)
      (:%20%20
        (if (== (Variables|Default|GetSpawn%20Index) 4)
          (Variables|Default|SetCard%20Spawn (Math|Transform|MakeTransform (Math|Vector|MakeVector (+ (.x (.location (Variables|Default|GetCard%20Spawn))) -4e+02) -245.0 (.z (.location (Variables|Default|GetCard%20Spawn)))) "0, 0, 0" "1.000000,1.000000,1.000000"))
          (Variables|Default|SetSpawn%20Index 0))))))

(event Custom|Two%20card%20choosen%20?
  (Math|Integer|IncrementInt (Variables|Default|GetCard%20Choosen%20?)
    (:%20%20
      (if (== (Variables|Default|GetCard%20Choosen%20?) 2)
        (Variables|/Script/Engine.PlayerController|SetbShowMouseCursor (Game|GetPlayerController 0) false)))))

(event Custom|Card%20verification
  (if (== (Variables|Default|GetCard%20Choosen%20?) 2)
    (if (not (== (Variables|/Game/Blueprints/BP_Memory.BP_Memory_C|GetCard%20Index (Utilities|Array|Get(acopy) (Variables|Default|GetCard%20List%20Choosen))) (Variables|/Game/Blueprints/BP_Memory.BP_Memory_C|GetCard%20Index (Utilities|Array|Get(acopy) (Variables|Default|GetCard%20List%20Choosen) 1))))
      (bind _open (Timeline|Return%20card ReverseFromEnd)
        (:Update
          (Transformation|SetRelativeRotation (Variables|/Game/Blueprints/BP_Memory.BP_Memory_C|GetDoor (Utilities|Array|Get(acopy) (Variables|Default|GetCard%20List%20Choosen))) (Math|Rotator|MakeRotator 0.0 0.0 _open) false false))
        (:Finished
          (Variables|/Script/Engine.PlayerController|SetbShowMouseCursor (Game|GetPlayerController 0) true)
          (Variables|Default|SetCard%20Choosen%20? 0)
          (Utilities|Array|Clear (Variables|Default|GetCard%20List%20Choosen)))))))

(event EventBeginPlay
  (bind _returnvalue (Game|GetPlayerController 0))
  (Variables|/Script/Engine.PlayerController|SetbShowMouseCursor _returnvalue true)
  (Variables|/Script/Engine.PlayerController|SetbEnableClickEvents _returnvalue true)
  (CallFunction|SpawnCard))

(fn ConstructionScript)